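; Trigger box Blueprint that shows a "Press "T" to talk" prompt on the HUD while an actor overlaps it.
; Begin and end overlap set the instruction text or empty it, then share one path that passes it to BasicHUD's DrawTextToScreen.
; Both events also set IsOverlapOver to true, but its branch does nothing and a DestroyComponent call is unconnected.
; It does not check which actor overlaps or handle the T key.
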(event `self.ReceiveActorBeginOverlap`
  (params (OtherActor :type "Actor Object Reference"))
  (set `self.instruction` "Press \"T\" to talk")
  (bind _asbasic_hud (cast `/Game/HUD/BasicHUD` (`PlayerController.GetHUD` (`GameplayStatics.GetPlayerController` 0)) :!label _label))
  (`/Game/HUD/BasicHUD.DrawTextToScreen` _asbasic_hud true (`self.instruction`))
  (bind _output_get (set `self.isOverlapOver` true :!label _label_2))
  (if _output_get
    _))

(event `self.ReceiveActorEndOverlap`
  (params (OtherActor :type "Actor Object Reference"))
  (set `self.instruction` "")
  (`|ExecutionSequence`
    (:`then_0`
      (goto _label))
    (:`then_1`
      (goto _label_2))))

(fn `UserConstructionScript`)