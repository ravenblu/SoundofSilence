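; NPC actor that holds a branching dialogue with the player, starting when the player character overlaps its box.
; It shows the current statement in a timed text widget that follows the NPC's projected screen position each tick, alongside a numbered response list.
; Keys 1–3 pick a response, triggering Talk on the ThirdPersonCharacter.
; Each response's GoToStatement index selects the next statement; non-positive indices or statements without responses close the options.
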(event OnComponentBeginOverlap(Box)
  (params (OtherActor :type Actor%20Object%20Reference) (OtherComp :type Primitive%20Component%20Object%20Reference) (OtherBodyIndex :type Integer) (bFromSweep :type Boolean) (SweepResult :type Hit%20Result%20Structure%20%28by%20ref%29))
  (if (== OtherActor (Game|GetPlayerCharacter 0))
    (Variables|Default|SetCurrentStatement 0)
    (CallFunction|ShowOptions)))

(event EventBeginPlay
  (CallFunction|CreateWidgets))

(event EventActorBeginOverlap
  (params (OtherActor :type Actor%20Object%20Reference)))

(event EventTick
  (params (DeltaSeconds :type Float%20%28single-precision%29))
  (CallFunction|UpdateWidget))

(event Input|KeyboardEvents|1
  (params (Key :type Key%20Structure :default "AnyKey"))
  (:Released
    (if (Variables|Default|GetWaitingForResponse)
      (if (>= (Utilities|Array|Length (.Player_Responses (Utilities|Struct|BreakStruct_NPCStatement (Utilities|Array|Get(acopy) (Variables|Default|GetNPCStatements) (Variables|Default|GetCurrentStatement))))) 1)
        (CallFunction|Respond)))))

(event Input|KeyboardEvents|2
  (params (Key :type Key%20Structure :default "AnyKey"))
  (:Released
    (if (Variables|Default|GetWaitingForResponse)
      (if (>= (Utilities|Array|Length (.Player_Responses (Utilities|Struct|BreakStruct_NPCStatement (Utilities|Array|Get(acopy) (Variables|Default|GetNPCStatements) (Variables|Default|GetCurrentStatement))))) 2)
        (CallFunction|Respond 1)))))

(event Input|KeyboardEvents|3
  (params (Key :type Key%20Structure :default "AnyKey"))
  (:Released
    (if (Variables|Default|GetWaitingForResponse)
      (if (>= (Utilities|Array|Length (.Player_Responses (Utilities|Struct|BreakStruct_NPCStatement (Utilities|Array|Get(acopy) (Variables|Default|GetNPCStatements) (Variables|Default|GetCurrentStatement))))) 3)
        (CallFunction|Respond 2)))))

(fn ConstructionScript)

(fn CreateWidgets
  (Utilities|FlowControl|Sequence
    (:then_0
      (bind _returnvalue (UserInterface|CreateWidget "/Game/NPCDialogueSystem/Blueprints/WB_DialogueText.WB_DialogueText_C"))
      (bind _output_get (Variables|Default|SetDialogueWidget _returnvalue))
      (UserInterface|Viewport|AddtoViewport _output_get 0)
      (Widget|SetVisibility _output_get "Hidden")
      (Class|UserWidget|SetDesiredSizeinViewport _output_get "(X=500.000000,Y=200.000000)")
      (Appearance|SetColorandOpacity (Variables|/Game/NPCDialogueSystem/Blueprints/WB_DialogueText.WB_DialogueText_C|GetDialogue _output_get) (Variables|Default|GetColor) :!class /Script/UMG.TextBlock))
    (:then_1
      (bind _returnvalue_2 (UserInterface|CreateWidget "/Game/NPCDialogueSystem/Blueprints/WB_PlayerOptions.WB_PlayerOptions_C"))
      (bind _output_get_2 (Variables|Default|SetOptionsWidget _returnvalue_2))
      (UserInterface|Viewport|AddtoViewport _output_get_2 0)
      (Widget|SetVisibility _output_get_2 "Hidden"))))

(fn Talk
  (params (Text :type String) (Time :type Float%20%28single-precision%29))
  (bind _dialoguewidget (Variables|Default|GetDialogueWidget))
  (Rendering|Components|TextRender|SetText (Variables|/Game/NPCDialogueSystem/Blueprints/WB_DialogueText.WB_DialogueText_C|GetDialogue _dialoguewidget) (Utilities|Text|ToText(String) Text))
  (Widget|SetVisibility _dialoguewidget "Visible")
  (Class|KismetSystemLibrary|ClearTimerHandle (Variables|Default|GetTimer))
  (Utilities|Time|SetTimerbyFunctionName 0 "ClearTalk" Time))

(fn ClearTalk
  (bind _dialoguewidget (Variables|Default|GetDialogueWidget))
  (Rendering|Components|TextRender|SetText (Variables|/Game/NPCDialogueSystem/Blueprints/WB_DialogueText.WB_DialogueText_C|GetDialogue _dialoguewidget) "")
  (Widget|SetVisibility _dialoguewidget "Hidden"))

(fn UpdateWidget
  (Class|UserWidget|SetPositioninViewport (Variables|Default|GetDialogueWidget) (- (.ScreenPosition (Class|WidgetLayoutLibrary|ProjectWorldLocationtoWidgetPosition (Game|GetPlayerController 0) (Transformation|GetWorldLocation (Variables|Default|GetNPC)))) "(X=250.000000,Y=600.000000)") false))

(fn ShowOptions
  (bind _currentstatement (Variables|Default|GetCurrentStatement))
  (bind _npcstatements (Variables|Default|GetNPCStatements))
  (bind _optionswidget (Variables|Default|GetOptionsWidget))
  (bind _item (Utilities|Array|Get(acopy) _npcstatements _currentstatement))
  (bind (_npc_dialogue _player_responses) (Utilities|Struct|BreakStruct_NPCStatement _item))
  (if (< _currentstatement (Utilities|Array|Length _npcstatements))
    (CallFunction|Talk _npc_dialogue 2.5)
    (for (_array_element _array_index) _player_responses
      (LocalVariables|SetPlayerOptions (Utilities|String|BuildString(Integer) (LocalVariables|GetPlayerOptions) " " (+ _array_index 1) (Utilities|String|Append ". " (.Player_Response (Utilities|Struct|BreakStruct_PlayerResponse _array_element))))))
    (Rendering|Components|TextRender|SetText (Variables|/Game/NPCDialogueSystem/Blueprints/WB_PlayerOptions.WB_PlayerOptions_C|GetOptions _optionswidget) (Utilities|Text|ToText(String) (LocalVariables|GetPlayerOptions)))
    (Widget|SetVisibility _optionswidget "Visible")
    (Variables|Default|SetWaitingForResponse true)))

(fn Respond
  (params (ResponseIndex :type Integer))
  (bind _asthird_person_character (Utilities|Casting|CastToThirdPersonCharacter (Game|GetPlayerCharacter 0)))
  (Default|Talk _asthird_person_character)
  (if (> (.Go_To_Statement (Utilities|Struct|BreakStruct_PlayerResponse (Utilities|Array|Get(acopy) (.Player_Responses (Utilities|Struct|BreakStruct_NPCStatement (Utilities|Array|Get(acopy) (Variables|Default|GetNPCStatements) (Variables|Default|GetCurrentStatement)))) ResponseIndex))) 0)
    (bind _output_get (Variables|Default|SetCurrentStatement (.Go_To_Statement (Utilities|Struct|BreakStruct_PlayerResponse (Utilities|Array|Get(acopy) (.Player_Responses (Utilities|Struct|BreakStruct_NPCStatement (Utilities|Array|Get(acopy) (Variables|Default|GetNPCStatements) (Variables|Default|GetCurrentStatement)))) ResponseIndex)))))
    (if (> (Utilities|Array|Length (.Player_Responses (Utilities|Struct|BreakStruct_NPCStatement (Utilities|Array|Get(acopy) (Variables|Default|GetNPCStatements) _output_get)))) 0)
      (CallFunction|ShowOptions)
      (else
        (CallFunction|Talk "" 3.0)
        (Variables|Default|SetWaitingForResponse false :!label _label)
        (Widget|SetVisibility (Variables|Default|GetOptionsWidget) "Hidden")))
    (else
      (goto _label))))